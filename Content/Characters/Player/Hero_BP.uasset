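; Player hero Blueprint that turns input into camera look, movement, jump and light or heavy attacks.
; A Rule component arbitrates move, jump and attack motion states, with attack and jump rule events registered at BeginPlay.
; Movement input yields a camera-relative vector that rotates the actor on sharp direction changes.
; Attacks focus Skill component lines; skill-end events and Anim_BP notifies end the corresponding motions.
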(event `InputAxis|Forward`
  (params (AxisValue :type "Float (single-precision)"))
  (bind _returnvalue (`self.GetActorForwardVector`))
  (bind _camera (`self.Camera`))
  ;[0.01042 0.00973 0.009941] Simple Movement
  (`self.CanMove` AxisValue
    (:`True`
      _)
    (:`False`
      _))
  (bind _output_get (set `self.MovementVector` (+ (* AxisValue (`SceneComponent.GetForwardVector` _camera)) (* (stale `InputAxis|Turn` AxisValue) (`SceneComponent.GetRightVector` _camera))) :!label _label))
  (`/MeleeCore/Blueprints/MotionRules/MotionRuler.Switch Motion BP` (`self.Rule`) "NewEnumerator8")
  (bind _returnvalue_2 (`KismetMathLibrary.Dot_VectorVector` _output_get _returnvalue))
  (bind _returnvalue_3 (`KismetMathLibrary.DegAcos` _returnvalue_2))
  (if (or (< _returnvalue_2 0.0) (> (`KismetMathLibrary.Abs` _returnvalue_3) 80.0))
    (if (> (.z (`KismetMathLibrary.Cross_VectorVector` _output_get _returnvalue)) 0.0)
      (`self.K2_SetActorRelativeRotation` (`KismetMathLibrary.MakeRotator` 0.0 0.0 _returnvalue_3))
      (else
        (`self.K2_SetActorRelativeRotation` (`KismetMathLibrary.MakeRotator` 0.0 0.0 (* _returnvalue_3 -1.0)))))))

(event `InputAxis|Turn`
  (params (AxisValue :type "Float (single-precision)"))
  ;[0.01042 0.00973 0.009941] Simple Movement
  (`self.CanMove` AxisValue
    (:`True`
      (goto _label))
    (:`False`
      (goto _label))))

(event `InputAxis|ViewTurn`
  (params (AxisValue :type "Float (single-precision)"))
  ;[0.01042 0.00973 0.009941] Simple Movement
  (`self.AddControllerYawInput` AxisValue))

(event `InputAxis|ViewHight`
  (params (AxisValue :type "Float (single-precision)"))
  ;[0.01042 0.00973 0.009941] Simple Movement
  (`self.AddControllerPitchInput` AxisValue))

(event `self.ReceiveBeginPlay`
  (bind _rule (`self.Rule`))
  ;[1 1 1] Init and bind events
  (`MeleeUtils.DetachWeapon` (`self.DetectMelee`) "Melee_RightHand" (`self.HandAttack`))
  (`/MeleeCore/Blueprints/MotionRules/MotionRuler.Update Basic Rule BP` _rule "NewEnumerator1" (make `MotionRuleEvent` (`|CreateDelegate` :!event `Check Attack`)))
  (`/MeleeCore/Blueprints/MotionRules/MotionRuler.Update Basic Rule BP` _rule "NewEnumerator4" (make `MotionRuleEvent` (`|CreateDelegate` :!event `Check Jump`)))
  (add `/MeleeCore/Blueprints/Skill/BP_Skill.OnSkillEnd` (`self.Skill`) (`|CreateDelegate` :!event `On Skill Ended`))
  (bind _asanim_bp (cast `/Game/Characters/Player/Anim_BP` (`SkeletalMeshComponent.GetAnimInstance` (`self.Mesh`))))
  (add `/Game/Characters/Player/Anim_BP.OnEndJumpEvent` _asanim_bp (delegate `self.AnimNotify_OnEndJump`))
  (add `/Game/Characters/Player/Anim_BP.OnEndMoveEvent` _asanim_bp (delegate `self.AnimNotify_OnEndMove`)))

(event `self.AnimNotify_OnEndMove`
  ;[1 1 1] Init and bind events
  (`/MeleeCore/Blueprints/MotionRules/MotionRuler.End Motion BP` (`self.Rule`) "NewEnumerator8"))

(event `self.AnimNotify_OnEndJump`
  ;[1 1 1] Init and bind events
  (`/MeleeCore/Blueprints/MotionRules/MotionRuler.End Motion BP` (`self.Rule`) "NewEnumerator4")
  (set `self.IsJumping` false))

(event `InputAction|LightAttack`
  (params (Key :type "Key Structure"))
  (:`Pressed`
    (bind _result (`/MeleeCore/Blueprints/MotionRules/MotionRuler.Is Switchable BP` (`self.Rule`) "NewEnumerator1"))
    (if _result
      (bind _result_2 (`/MeleeCore/Blueprints/Skill/BP_Skill.Focus Skill Line BP` (`self.Skill`) "NewEnumerator0"))
      (if _result_2
        (`/MeleeCore/Blueprints/MotionRules/MotionRuler.Switch Motion BP` (`self.Rule`) "NewEnumerator1")))))

(event `InputAction|HeaveyAttack`
  (params (Key :type "Key Structure"))
  (:`Pressed`
    (`/MeleeCore/Blueprints/Skill/BP_Skill.Focus Skill Line BP` (`self.Skill`) "NewEnumerator1")))

(event `InputAction|Jump`
  (params (Key :type "Key Structure"))
  (bind _rule (`self.Rule`))
  (:`Pressed`
    (bind _result (`/MeleeCore/Blueprints/MotionRules/MotionRuler.Is Switchable BP` _rule "NewEnumerator4"))
    (if _result
      (set `self.IsJumping` true)
      (`/MeleeCore/Blueprints/MotionRules/MotionRuler.Switch Motion BP` _rule "NewEnumerator4"))))

(fn `Check Attack`
  (returns (ReturnValue :type Boolean))
  (bind _result (`/MeleeCore/Blueprints/Skill/BP_Skill.Can Switch from BP` (`self.Skill`) (make `/MeleeCore/Blueprints/Skill/BP_SkillTypes` (`|MakeArray` "NewEnumerator0" "NewEnumerator1" :!type "/MeleeCore/Blueprints/Skill/BP_SkillLineType Enum")) false))
  (return _result))

(fn `Check Jump`
  (returns (returnValue :type Boolean))
  (return (not (`self.IsJumping`))))

(fn `On Skill Ended`
  (params (skilllineName :type "/MeleeCore/Blueprints/Skill/BP_SkillLineType Enum" :default "NewEnumerator0"))
  (switch `/MeleeCore/Blueprints/Skill/BP_SkillLineType` skilllineName
    (:`NewEnumerator0`
      _)
    (:`NewEnumerator1`
      _))
  (`/MeleeCore/Blueprints/MotionRules/MotionRuler.End Motion BP` (`self.Rule`) "NewEnumerator1"))

(fn `UserConstructionScript`)