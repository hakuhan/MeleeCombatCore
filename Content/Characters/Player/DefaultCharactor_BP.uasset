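; Player character Blueprint with axis-driven movement and camera control, plus light and heavy melee attack input.
; CaMove and CanCombat macros gate movement and attacks using the cached Anim_BP's Locomotion/Combo state and flags set by UpdateMoveState and UpdateInputState events.
; Melee hit events print the hit type and spawn first-hit or multi-hit particles at the impact location.
; Combo end flags a stop and halts movement; the Tick state switch does nothing.
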(event `self.ReceiveBeginPlay`
  ;[1 1 1] Init
  (bind _asanim_bp (cast `/Game/Characters/Player/Anim_BP` (`SkeletalMeshComponent.GetAnimInstance` (`self.Mesh`))))
  (set `self.anim` _asanim_bp))

(event `InputAxis|Forward`
  (params (AxisValue :type "Float (single-precision)"))
  ;[1 1 1] Move
  (`self.CaMove`
    (:`yes`
      (`self.AddMovementInput` (`KismetMathLibrary.GetForwardVector` (`KismetMathLibrary.MakeRotator` 0.0 0.0 (.yaw (`self.GetControlRotation`)))) AxisValue))))

(event `InputAxis|ViewHight`
  (params (AxisValue :type "Float (single-precision)"))
  ;[1 1 1] Rotate camera
  (`self.AddControllerPitchInput` (* AxisValue 0.5)))

(event `InputAxis|ViewTurn`
  (params (AxisValue :type "Float (single-precision)"))
  ;[1 1 1] Rotate camera
  (`self.AddControllerYawInput` AxisValue))

(event `InputAxis|Turn`
  (params (AxisValue :type "Float (single-precision)"))
  ;[1 1 1] Move
  (`self.CaMove`
    (:`yes`
      (`self.AddMovementInput` (`KismetMathLibrary.GetRightVector` (`KismetMathLibrary.MakeRotator` 0.0 0.0 (.yaw (`self.GetControlRotation`)))) AxisValue))))

(event `InputAction|LightAttack`
  (params (Key :type "Key Structure"))
  ;[1 1 1] Attack
  (:`Pressed`
    (`self.CanCombat`
      (:`yes`
        (set `self.lightAttack` true))))
  (:`Released`
    (set `self.lightAttack` false)))

(event `InputAction|HeaveyAttack`
  (params (Key :type "Key Structure"))
  ;[1 1 1] Attack
  (:`Pressed`
    (`self.CanCombat`
      (:`yes`
        (set `self.heaveAttack` true))))
  (:`Released`
    (set `self.heaveAttack` false)))

(event `self.OnMeleeHitEffect`
  (params (hitInfo :type "HitResult Structure") (hitType :type "ECombatHitResult Enum" :default "NO_HIT"))
  (`KismetSystemLibrary.PrintString` (`|GetEnumeratorNameAsString` hitType))
  (`self.PlayHitEffect` hitInfo (`self.MultiHitEffect`)))

(event `self.OnMeleeFirstHitEffect`
  (params (hitInfo :type "HitResult Structure") (hitType :type "ECombatHitResult Enum" :default "NO_HIT"))
  (`KismetSystemLibrary.PrintString` (`|GetEnumeratorNameAsString` hitType))
  (`self.PlayHitEffect` hitInfo (`self.StartEffect`)))

(event `MeleeMoveInterface.UpdateMoveState`
  (params (canMove :type Boolean))
  ;[1 1 1] Combat notice
  (set `self.canCombattingMove` canMove))

(event `MeleeInputInterface.UpdateInputState`
  (params (canInput :type Boolean))
  ;[1 1 1] Combat notice
  (set `self.canCombattingInput` canInput))

(event `self.ReceiveTick`
  (params (DeltaSeconds :type "Float (single-precision)"))
  (bind _anim (`self.anim`))
  ;[1 1 1] Check combat state
  (`/Engine/EditorBlueprintResources/StandardMacros.IsValid` _anim
    (:`Is Valid`
      (switch `/Game/Tables/E_PlayerCombatAniState` (`/Game/Characters/Player/Anim_BP.State` _anim)))))

(event `MeleeComboInterface.OnComboOver`
  (bind _charactermovement (`self.CharacterMovement`))
  ;[1 1 1] Check combat state
  (set `self.comboStop` true)
  (set `MovementComponent.Velocity` (0.0 0.0 0.0) _charactermovement)
  (`MovementComponent.StopMovementImmediately` _charactermovement))

(fn `PlayHitEffect`
  (params (hit :type "HitResult Structure") (particle :type "ParticleSystem Object Reference"))
  (`/Engine/EditorBlueprintResources/StandardMacros.IsValid` particle
    (:`Is Valid`
      (`GameplayStatics.SpawnEmitterAtLocation` particle (`.Location` (`GameplayStatics.BreakHitResult` hit)) (struct) (1.0 1.0 1.0) true "AutoRelease"))))

(fn `UserConstructionScript`)